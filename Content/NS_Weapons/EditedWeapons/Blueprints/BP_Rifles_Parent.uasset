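; Parent rifle Blueprint that handles weapon animations and configurable skins for a skeletal mesh.
; Fire plays the fire animation when its selector is 1, and Reloading picks a hip, ironsight or prone animation by pose; both print debug text.
; The construction script chooses old or new materials, then pushes emissive, custom color and metallic parameters to them.
; Projectile spawning at the muzzle socket is present but unconnected, so firing spawns nothing.
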(event `Fire`
  (switch `int` (`self.FireAnimationNumber`)
    (:`1`
      (`SkeletalMeshComponent.PlayAnimation` (`self.SkeletalMesh`) "/Game/EditedWeapons/Animations/Fire_Anim.Fire_Anim" false)
      (`KismetSystemLibrary.PrintString` "FIRE" true true (struct :`R` 1.0 :`G` 0.067435 :`A` 1.0)))))

(event `Reloading`
  (bind _skeletalmesh (`self.SkeletalMesh`))
  (switch `/Game/EditedWeapons/DemoFolder/PreviewCharacterLogic/Blueprints/ENUM_PoseSelection` (`self.PoseSelection`)
    (:`NewEnumerator0`
      (`SkeletalMeshComponent.PlayAnimation` _skeletalmesh "/Game/EditedWeapons/Animations/Hip_Anim.Hip_Anim" false))
    (:`NewEnumerator1`
      (`SkeletalMeshComponent.PlayAnimation` _skeletalmesh "/Game/EditedWeapons/Animations/Ironsight_Anim.Ironsight_Anim" false))
    (:`NewEnumerator2`
      (`SkeletalMeshComponent.PlayAnimation` _skeletalmesh "/Game/EditedWeapons/Animations/Prone_Anim.Prone_Anim" false)))
  (`KismetSystemLibrary.PrintString` "RELOADING" true true (struct :`R` 0.090979 :`G` 1.0 :`A` 1.0)))

(fn `UserConstructionScript`
  (bind _skeletalmesh (`self.SkeletalMesh`))
  (bind _skeletalmesh_2 (`self.SkeletalMesh`))
  (bind _skeletalmesh_3 (`self.SkeletalMesh`))
  (bind _skeletalmesh_4 (`self.SkeletalMesh`))
  (`|ExecutionSequence`
    (:`then_0`
      (if (`self.isOldMaterial`)
        (`PrimitiveComponent.SetMaterial` _skeletalmesh_3 0 (`self.OldMaterial00`))
        (`PrimitiveComponent.SetMaterial` _skeletalmesh_3 1 (`self.OldMaterial01`))
        (else
          (`PrimitiveComponent.SetMaterial` _skeletalmesh_2 0 (`self.NewMaterial00`))
          (`PrimitiveComponent.SetMaterial` _skeletalmesh_2 1 (`self.NewMaterial01`)))))
    (:`then_1`
      (`MeshComponent.SetScalarParameterValueOnMaterials` _skeletalmesh_4 "EmissivePower" (`self.EmissivePover`)))
    (:`then_2`
      (`MeshComponent.SetVectorParameterValueOnMaterials` _skeletalmesh_4 "EmissiveColor" (`KismetMathLibrary.Conv_LinearColorToVector` (`self.EmissiveColor`))))
    (:`then_3`
      (`MeshComponent.SetScalarParameterValueOnMaterials` _skeletalmesh "isCustomColors" (`KismetMathLibrary.Conv_BoolToDouble` (`self.isCustomColors`)))
      (`MeshComponent.SetVectorParameterValueOnMaterials` _skeletalmesh "Color01" (`KismetMathLibrary.Conv_LinearColorToVector` (`self.Color01`)))
      (`MeshComponent.SetVectorParameterValueOnMaterials` _skeletalmesh "Color02" (`KismetMathLibrary.Conv_LinearColorToVector` (`self.Color02`)))
      (`MeshComponent.SetVectorParameterValueOnMaterials` _skeletalmesh "Color03" (`KismetMathLibrary.Conv_LinearColorToVector` (`self.Color03`)))
      (`MeshComponent.SetVectorParameterValueOnMaterials` _skeletalmesh "Color04" (`KismetMathLibrary.Conv_LinearColorToVector` (`self.Color04`)))
      (`MeshComponent.SetVectorParameterValueOnMaterials` _skeletalmesh "MetallicColor" (`KismetMathLibrary.Conv_LinearColorToVector` (`self.MetallicColor`))))))