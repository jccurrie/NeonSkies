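; Parent rifle Blueprint from a weapon bundle's demo preview logic, with customizable material colors and simple Fire and Reloading events.
; The construction script pushes emissive, color, metallic color and custom-color toggle variables to the skeletal mesh's materials.
; Fire and Reloading each call a non-looping mesh animation and print a debug message.
; A muzzle-socket projectile spawn leading into the Fire logic is left unconnected, so it never runs.
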(event `Fire`
  (`SkeletalMeshComponent.PlayAnimation` (`self.SkeletalMesh`) null false)
  (`KismetSystemLibrary.PrintString` "FIRE" true true (struct :`R` 1.0 :`G` 0.067435 :`A` 1.0)))

(event `Reloading`
  (`SkeletalMeshComponent.PlayAnimation` (`self.SkeletalMesh`) null false)
  (`KismetSystemLibrary.PrintString` "RELOADING" true true (struct :`R` 0.090979 :`G` 1.0 :`A` 1.0)))

(fn `UserConstructionScript`
  (bind _skeletalmesh (`self.SkeletalMesh`))
  (bind _skeletalmesh_2 (`self.SkeletalMesh`))
  (`|ExecutionSequence`
    (:`then_0`
      (`MeshComponent.SetScalarParameterValueOnMaterials` _skeletalmesh "EmissivePower" (`self.EmissivePover`)))
    (:`then_1`
      (`MeshComponent.SetVectorParameterValueOnMaterials` _skeletalmesh "EmissiveColor" (`KismetMathLibrary.Conv_LinearColorToVector` (`self.EmissiveColor`))))
    (:`then_2`
      (`MeshComponent.SetVectorParameterValueOnMaterials` _skeletalmesh_2 "Color01" (`KismetMathLibrary.Conv_LinearColorToVector` (`self.Color01`)))
      (`MeshComponent.SetVectorParameterValueOnMaterials` _skeletalmesh_2 "Color02" (`KismetMathLibrary.Conv_LinearColorToVector` (`self.Color02`)))
      (`MeshComponent.SetVectorParameterValueOnMaterials` _skeletalmesh_2 "Color03" (`KismetMathLibrary.Conv_LinearColorToVector` (`self.Color03`)))
      (`MeshComponent.SetVectorParameterValueOnMaterials` _skeletalmesh_2 "MetallicColor" (`KismetMathLibrary.Conv_LinearColorToVector` (`self.MetallicColor`))))
    (:`then_3`
      (`MeshComponent.SetScalarParameterValueOnMaterials` _skeletalmesh_2 "isCustomColors" (`KismetMathLibrary.Conv_BoolToDouble` (`self.isCustomColors`))))))